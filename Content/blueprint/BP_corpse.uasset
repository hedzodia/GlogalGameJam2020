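; BP_corpse is a corpse actor that makes a sound and leaves blood splatters when it is moved.
; HasBeenMoved plays a random body-grab Wwise event, then spawns a random number of BP_Splatter actors within a flat box around the corpse at a fixed world height.
; Each spawn plays a splash sound on the player and registers the splatter in the first-person character's BloodSplattersArray, using the reference cached at BeginPlay.
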(event `self.ReceiveBeginPlay`
  (set `self.player` (cast `/Game/FirstPersonBP/Blueprints/FirstPersonCharacter` (`GameplayStatics.GetPlayerCharacter` 0) :!pure true)))

(event `HasBeenMoved`
  (bind (_returnvalue_x _returnvalue_y) (`KismetMathLibrary.BreakVector` (`KismetMathLibrary.RandomPointInBoundingBox` (`self.K2_GetActorLocation`) (50.0 50.0 0.0))))
  (`AkGameplayStatics.PostEvent` "/Game/Audio/Objects/Play_GrabBody_RND.Play_GrabBody_RND" (`ActorComponent.GetOwner` (`self.SkeletalMesh`)))
  (for _ (range (+ (`KismetMathLibrary.RandomIntegerInRange` (`self.#MinBloodStains`) (`self.#MaxBloodStains`)) 1))
    (bind _returnvalue (`|SpawnActorFromClass` "/Game/blueprint/BP_Splatter.BP_Splatter_C" (`KismetMathLibrary.MakeTransform` (`KismetMathLibrary.MakeVector` _returnvalue_x _returnvalue_y 170.0) (struct) (0.05 0.05 3.0)) "Undefined" "OverrideRootScale" null null))
    (`AkGameplayStatics.PostEvent` "/Game/Audio/Other/Play_Blood_Splash_RND.Play_Blood_Splash_RND" (`self.player`))
    (`KismetArrayLibrary.Array_AddUnique` (`/Game/FirstPersonBP/Blueprints/FirstPersonCharacter.BloodSplattersArray` (`self.player`)) _returnvalue)))

(fn `UserConstructionScript`)
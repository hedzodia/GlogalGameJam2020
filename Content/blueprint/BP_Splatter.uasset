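; BP_Splatter is a blood splatter actor the player cleans with a sponge.
; On BeginPlay it spawns a randomly sized decal along its up vector, using a dynamic material with a random frame for variety.
; Each box overlap by a usable BP_Sponge while the player sponges plays a cleaning sound and decrements CleanCount.
; At zero it removes decal and actor, then notifies the player and sponge.
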(event `self.ReceiveBeginPlay`
  (`|ExecutionSequence`
    (:`then_0`
      (set `self.player` (cast `/Game/FirstPersonBP/Blueprints/FirstPersonCharacter` (`GameplayStatics.GetPlayerCharacter` 0) :!pure true)))
    (:`then_1`
      (bind _returnvalue (`KismetMaterialLibrary.CreateDynamicMaterialInstance` "/Game/BloodStains/splatters_decal_M.splatters_decal_M"))
      (`MaterialInstanceDynamic.SetScalarParameterValue` _returnvalue "Frame" (`KismetMathLibrary.Conv_IntToDouble` (`KismetMathLibrary.RandomInteger` 11)))
      (bind _returnvalue_2 (`GameplayStatics.SpawnDecalAtLocation` _returnvalue (`KismetMathLibrary.Conv_DoubleToVector` (`KismetMathLibrary.RandomFloatInRange` 20.0 50.0)) (`self.K2_GetActorLocation`) (`KismetMathLibrary.Conv_VectorToRotator` (`self.GetActorUpVector`))))
      (set `self.décaloté` _returnvalue_2))))

(event `self.Box.OnComponentBeginOverlap`
  (params (OverlappedComponent :type "PrimitiveComponent Object Reference") (OtherActor :type "Actor Object Reference") (OtherComp :type "PrimitiveComponent Object Reference") (OtherBodyIndex :type Integer) (bFromSweep :type Boolean) (SweepResult :type "HitResult Structure (by ref)"))
  (bind _asbp_sponge (cast `/Game/blueprint/BP_Sponge` OtherActor))
  (if (`/Game/blueprint/BP_Sponge.canClean` _asbp_sponge)
    (if (`/Game/FirstPersonBP/Blueprints/FirstPersonCharacter.usingSponge` (cast `/Game/FirstPersonBP/Blueprints/FirstPersonCharacter` (`GameplayStatics.GetPlayerCharacter` 0) :!pure true))
      (`AkGameplayStatics.PostEvent` "/Game/Audio/Sponge/Play_SFX_SpongeCleaning_Loop.Play_SFX_SpongeCleaning_Loop" (`self.player`))
      (`KismetSystemLibrary.PrintString` "Cleaning")
      (bind _output_get (set `self.cleanCount` (- (`self.cleanCount`) 1)))
      (if (<= _output_get 0)
        (`ActorComponent.K2_DestroyComponent` (`self.décaloté`))
        (`self.K2_DestroyActor`)
        (`/Game/FirstPersonBP/Blueprints/FirstPersonCharacter.RemoveBloodFromArray` (`self.player`) self)
        (`/Game/blueprint/BP_Sponge.CleanedBlood` _asbp_sponge)))))

(fn `UserConstructionScript`)
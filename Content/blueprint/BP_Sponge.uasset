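; BP_Sponge is a cleaning sponge that can remove blood a limited number of times before it must be wrung out.
; Each CleanedBlood call decrements UsesLeft, and at zero it disables CanClean and swaps the Cube mesh to the dirty material.
; WringSponge restores uses and the clean material, and posts a Wwise wringing sound at a hardcoded world location rather than at the sponge.
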(event `self.ReceiveBeginPlay`
  (set `self.usesLeft` (`self.maxUses`))
  (`PrimitiveComponent.SetMaterial` (`self.Cube`) 0 (`self.textureClean`)))

(event `CleanedBlood`
  (bind _result (`/Engine/EditorBlueprintResources/StandardMacros.DecrementInt` (`self.usesLeft`))
    (:`  `
      (if (<= _result 0)
        (set `self.canClean` false)
        (`PrimitiveComponent.SetMaterial` (`self.Cube`) 0 (`self.textureDirty`))))))

(event `WringSponge`
  (`AkGameplayStatics.PostEventAtLocation` "/Game/Audio/Sponge/Play_Essorage_RND.Play_Essorage_RND" (-970.0 790.0 270.0))
  (set `self.canClean` true)
  (set `self.usesLeft` (`self.maxUses`))
  (`PrimitiveComponent.SetMaterial` (`self.Cube`) 0 (`self.textureClean`)))

(fn `UserConstructionScript`)